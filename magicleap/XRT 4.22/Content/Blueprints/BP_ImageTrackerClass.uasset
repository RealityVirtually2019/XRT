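; Blueprint actor that wraps an ImageTracker component for tracking a target image.
; On BeginPlay it copies its own settings onto the component: target texture, tracker name, physical size, stationary flag and unreliable-pose option.
; Simple getter functions expose those same settings to other Blueprints.
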(event `self.ReceiveBeginPlay`
  (bind _imagetracker (`self.ImageTracker`))
  ;[0.165 1 0.1379] Initialize
  (set `ImageTrackerComponent.TargetImageTexture` (`self.TargetImageTexture`) _imagetracker)
  (set `ImageTrackerComponent.Name` (`self.TrackerName`) _imagetracker)
  (set `ImageTrackerComponent.LongerDimension` (`self.LongerDimension`) _imagetracker)
  (set `ImageTrackerComponent.bIsStationary` (`self.IsImageTargetStationary`) _imagetracker)
  (set `ImageTrackerComponent.bUseUnreliablePose` (`self.UseUnreliablePose`) _imagetracker))

(fn `GetIsImageTargetStationary`
  (returns (IsStationary :type Boolean))
  (return (`self.IsImageTargetStationary`)))

(fn `GetLongerDimension`
  (returns (LongerDimension :type "Float (double-precision)"))
  (return (`self.LongerDimension`)))

(fn `GetTargetImageTexture`
  (returns (Image :type "Texture2D Object Reference"))
  (return (`self.TargetImageTexture`)))

(fn `GetTrackerName`
  (returns (Name :type String))
  (return (`self.TrackerName`)))

(fn `GetUseUnreliablePose`
  (returns (Enabled :type Boolean))
  (return (`self.UseUnreliablePose`)))

(fn `UserConstructionScript`)