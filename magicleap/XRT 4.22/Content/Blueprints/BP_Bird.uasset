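; Bird actor that perches on the player's index fingertip via hand-gesture tracking and flies away when the gesture is lost.
; BeginPlay configures the gesture set and filtering, then Tick polls either hand's current gesture.
; A Finger gesture plays the looping flight animation and snaps the skeletal mesh to the fingertip.
; Once tracked, NoPose or NoHand restarts a timeline that lerps the mesh toward a fixed world point.
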(event `self.ReceiveBeginPlay`
  (bind _returnvalue (`MagicLeapHandTrackingFunctionLibrary.SetConfiguration` (`|MakeArray` "Finger" "NoPose" "NoHand" "OpenHandBack" "L" :!type "EHandTrackingGesture Enum") "SimpleSmoothing" "MoreRobustnessToFlicker"))
  (`KismetSystemLibrary.PrintString` (`KismetStringLibrary.Conv_BoolToString` _returnvalue)))

(event `self.ReceiveTick`
  (params (DeltaSeconds :type "Float (single-precision)"))
  (bind _gesture (`MagicLeapHandTrackingFunctionLibrary.GetCurrentGesture` "AnyHand"))
  (`KismetSystemLibrary.PrintString` (`|GetEnumeratorNameAsString` _gesture))
  (switch `EHandTrackingGesture` _gesture
    (:`Finger`
      (`SkeletalMeshComponent.PlayAnimation` (`self.SkeletalMesh`) "/Game/Models/AnimatedBird/Animations/flyfly/flying_Anim.flying_Anim" true)
      (bind _transform (`MagicLeapHandTrackingFunctionLibrary.GetGestureKeypointTransform` "AnyHand" "Index_Tip" "World"))
      (`KismetSystemLibrary.PrintString` (`KismetStringLibrary.Conv_TransformToString` _transform))
      (`SceneComponent.K2_SetWorldTransform` (`self.SkeletalMesh`) (`KismetMathLibrary.MakeTransform` (.location _transform) (.rotation _transform)) false false)
      (set `self.IsBirdTracked` true))
    (:`NoPose`
      (if (`self.IsBirdTracked`) :!label _label
        (bind (_direction _birdflyaway) (`Timeline|Timeline_0` :!via `PlayFromStart`)
          (:`Update`
            (`SceneComponent.K2_SetWorldTransform` (`self.SkeletalMesh`) (`KismetMathLibrary.MakeTransform` (`KismetMathLibrary.VLerp` (`SceneComponent.K2_GetComponentLocation` (`self.SkeletalMesh`)) (200.0 200.0 200.0) _birdflyaway) (`SceneComponent.K2_GetComponentRotation` (`self.SkeletalMesh`))) true false)))))
    (:`NoHand`
      (goto _label))))

(fn `UserConstructionScript`)