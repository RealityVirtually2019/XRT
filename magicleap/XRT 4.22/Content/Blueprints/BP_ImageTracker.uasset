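; Image tracker controller that shows an art-specific visualizer (lotus scene for Chinese Painting, Starry Night visualizer) on the tracked image.
; Binds found, lost and unreliable tracker events to set tracking status and write it to an information panel.
; While tracking is reliable, Tick selects the visualizer by tracker name and follows the image's pose behind threshold checks.
; Lost and unreliable handlers act on a separate tracked-object reference, not the current visualizer.
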(event `OnTargetLost`
  ;[1 0.7298 0.3146] Tick
  ;;[0.165 1 0.1379] Initialize
  ;;;[1 1 1] Handle image tracking events
  (`self.OnImageTargetLost`))

(event `self.ReceiveBeginPlay`
  (bind _imagetracker (`/Game/Blueprints/BP_ImageTrackerClass.ImageTracker` (`self.ImageTrackerReference`)))
  ;[0.165 1 0.1379] Initialize
  (`|ExecutionSequence`
    (:`then_0`
      ;[1 0.7298 0.3146] Tick
      (`/Game/Examples/Blueprints/Utility/InformationPanel.SetTextAtIndex` (`self.InformationPanel`) (`self.InformationPanelTrackerIndex`) (`KismetTextLibrary.Conv_StringToText` (`KismetStringLibrary.Concat_StrStr` (`/Game/Blueprints/BP_ImageTrackerClass.GetTrackerName` (`self.ImageTrackerReference`)) "Status:"))))
    (:`then_1`
      ;;;[1 1 1] Handle image tracking events
      (add `ImageTrackerComponent.OnImageTargetFound` _imagetracker (delegate `OnTargetFound`))
      (add `ImageTrackerComponent.OnImageTargetLost` _imagetracker (delegate `OnTargetLost`))
      (add `ImageTrackerComponent.OnImageTargetUnreliableTracking` _imagetracker (delegate `OnTargetUnreliable`)))))

(event `OnTargetFound`
  ;[1 0.7298 0.3146] Tick
  ;;[0.165 1 0.1379] Initialize
  ;;;[1 1 1] Handle image tracking events
  (`self.OnImageTargetFound`))

(event `OnTargetUnreliable`
  (params (LastTrackedLocation :type "Vector Structure (by ref)") (LastTrackedRotation :type "Rotator Structure (by ref)") (NewUnreliableLocation :type "Vector Structure (by ref)") (NewUnreliableRotation :type "Rotator Structure (by ref)"))
  ;[1 0.7298 0.3146] Tick
  ;;[0.165 1 0.1379] Initialize
  ;;;[1 1 1] Handle image tracking events
  (`self.OnImageTargetUnreliable` LastTrackedLocation LastTrackedRotation NewUnreliableLocation NewUnreliableRotation))

(event `self.ReceiveTick`
  (params (DeltaSeconds :type "Float (single-precision)"))
  (bind _currentvisualizer (`self.CurrentVisualizer`))
  (bind _currentvisualizer_2 (`self.CurrentVisualizer`))
  (bind _currentvisualizer_3 (`self.CurrentVisualizer`))
  (bind _oldvisualizer (`self.OldVisualizer`))
  (bind _imagetracker (`/Game/Blueprints/BP_ImageTrackerClass.ImageTracker` (`self.ImageTrackerReference`)))
  (bind _returnvalue (`SceneComponent.K2_GetComponentRotation` _imagetracker))
  (bind _returnvalue_2 (`KismetMathLibrary.MakeVector` (+ (.x (`SceneComponent.K2_GetComponentLocation` _imagetracker)) 0.0) (- (.y (`SceneComponent.K2_GetComponentLocation` _imagetracker)) 0.0) (+ (.z (`SceneComponent.K2_GetComponentLocation` _imagetracker)) 0.0)))
  ;[1 0.7298 0.3146] Tick
  (`|ExecutionSequence`
    (:`then_0`
      (if (`KismetSystemLibrary.IsValid` _oldvisualizer)
        ;;[0.165 1 0.1379] Initialize
        (`self.SetActorHiddenInGame` _oldvisualizer true)))
    (:`then_1`
      (`KismetSystemLibrary.Delay` 0.0)
      (`self.UpdateViewModeText`)
      (if (`|EnumEquality` (`self.TrackingStatus`) "NewEnumerator1")
        (`|ExecutionSequence`
          (:`then_0`
            (switch `string` (`/Game/Blueprints/BP_ImageTrackerClass.GetTrackerName` (`self.ImageTrackerReference`))
              (:`ChinesePainting`
                (bind _outactors (`GameplayStatics.GetAllActorsOfClass` "/Game/Blueprints/Visualizers/BP_LotusVisualizer.BP_LotusVisualizer_C"))
                (`|ExecutionSequence`
                  (:`then_0`
                    (bind _output (`|GetArrayItem` _outactors))
                    (set `self.DidVisualizerChange` (!= _currentvisualizer_2 _output))
                    (set `self.OldVisualizer` _currentvisualizer_2))
                  (:`then_1`
                    (bind _output_get (set `self.CurrentVisualizer` _output))
                    (`self.SetActorHiddenInGame` _output_get false)
                    (`/Game/Blueprints/Visualizers/BP_LotusVisualizer.ResetLotus` _output))))
              (:`StarryNight`
                (bind _outactors_2 (`GameplayStatics.GetAllActorsOfClass` "/Game/Blueprints/Visualizers/BP_StarryNightVisualizer.BP_StarryNightVisualizer_C"))
                (`|ExecutionSequence`
                  (:`then_0`
                    (bind _output_2 (`|GetArrayItem` _outactors_2))
                    (set `self.DidVisualizerChange` (!= _currentvisualizer_3 _output_2))
                    (set `self.OldVisualizer` _currentvisualizer_3))
                  (:`then_1`
                    (bind _output_get_2 (set `self.CurrentVisualizer` _output_2))
                    (`self.SetActorHiddenInGame` _output_get_2 false))))))
          (:`then_1`
            (bind _returnvalue_3 (`self.K2_GetActorLocation` _output_get))
            (if (or (>= (.x (`KismetMathLibrary.Normal` (- _returnvalue_2 _returnvalue_3))) 0.3) (>= (.y (`KismetMathLibrary.Normal` (- _returnvalue_2 _returnvalue_3))) 0.3) (>= (.z (`KismetMathLibrary.Normal` (- _returnvalue_2 _returnvalue_3))) 0.3))
              (`self.K2_SetActorLocation` _currentvisualizer (`KismetMathLibrary.VLerp` _returnvalue_2 _returnvalue_3 DeltaSeconds) true false)))
          (:`then_2`
            ;;[1 1 1] Move object to tracked location and rotation
            (if true
              _))
          (:`then_3`
            (if (or (>= (- (.roll _returnvalue) (.roll (`self.K2_GetActorRotation` _currentvisualizer))) 0.7) (>= (- (.pitch _returnvalue) (.pitch (`self.K2_GetActorRotation` _currentvisualizer))) 0.7) (>= (- (.yaw _returnvalue) (.yaw (`self.K2_GetActorRotation` _currentvisualizer))) 0.7))
              (`self.K2_SetActorRotation` _currentvisualizer _returnvalue false))))))))

(fn `GetCurrentTrackingStatus`
  (returns (Status :type "/Game/Examples/Enums/E_ImageTrackingStatus Enum"))
  (return (`self.TrackingStatus`)))

(fn `OnImageTargetFound`
  (bind _imagetrackerreference (`self.ImageTrackerReference`))
  (bind _oldvisualizer (`self.OldVisualizer`))
  (bind _oldvisualizer_2 (`self.OldVisualizer`))
  (bind _imagetracker (`/Game/Blueprints/BP_ImageTrackerClass.ImageTracker` _imagetrackerreference))
  (`|ExecutionSequence`
    (:`then_0`
      (set `self.TrackingStatus` "NewEnumerator1"))
    (:`then_1`
      ;[1 1 1] Change text based on tracking state
      (`/Game/Examples/Blueprints/Utility/InformationPanel.SetTextAtIndex` (`self.InformationPanel`) (`self.InformationPanelTrackerIndex`) (`|FormatText` "{name} Status: Target Found (Reliable)" (`KismetTextLibrary.Conv_StringToText` (`/Game/Blueprints/BP_ImageTrackerClass.GetTrackerName` (`self.ImageTrackerReference`))))))
    (:`then_2`
      ;[1 1 1] Move tracked object to where the image was found
      (`|ExecutionSequence`
        (:`then_0`
          (switch `string` (`/Game/Blueprints/BP_ImageTrackerClass.GetTrackerName` _imagetrackerreference)
            (:`StarryNight`
              (`KismetSystemLibrary.PrintString` "Found Starry Night")
              (bind _outactors (`GameplayStatics.GetAllActorsOfClass` "/Game/Blueprints/Visualizers/BP_StarryNightVisualizer.BP_StarryNightVisualizer_C"))
              (set `self.CurrentVisualizer` (`|GetArrayItem` _outactors))
              (if (`KismetSystemLibrary.IsValid` _oldvisualizer_2)
                (`self.SetActorHiddenInGame` _oldvisualizer_2 true)))
            (:`ChinesePainting`
              (`KismetSystemLibrary.PrintString` "Found China")
              (bind _outactors_2 (`GameplayStatics.GetAllActorsOfClass` "/Game/Blueprints/Visualizers/BP_LotusVisualizer.BP_LotusVisualizer_C"))
              (bind _output (`|GetArrayItem` _outactors_2))
              (set `self.CurrentVisualizer` _output)
              (if (`KismetSystemLibrary.IsValid` _oldvisualizer)
                (`self.SetActorHiddenInGame` _oldvisualizer true))
              (`/Engine/EditorBlueprintResources/StandardMacros.DoOnce` false
                (:`Completed`
                  (`/Game/Blueprints/Visualizers/BP_LotusVisualizer.BeginLotusSceneEvent` _output))))))
        (:`then_1`
          (`self.K2_SetActorLocationAndRotation` (`self.CurrentVisualizer`) (`SceneComponent.K2_GetComponentLocation` _imagetracker) (select `bool` (`self.RotateTrackedObject`) :`false` (`self.K2_GetActorRotation` (`self.TrackedObjectReference`)) :`true` (`SceneComponent.K2_GetComponentRotation` _imagetracker)) false false))))
    (:`then_3`
      ;[1 1 1] Make tracked object visible
      (`self.SetActorHiddenInGame` (`self.CurrentVisualizer`) false))))

(fn `OnImageTargetLost`
  (`|ExecutionSequence`
    (:`then_0`
      (set `self.TrackingStatus` "NewEnumerator3"))
    (:`then_1`
      ;[1 1 1] Change text based on tracking state
      (`/Game/Examples/Blueprints/Utility/InformationPanel.SetTextAtIndex` (`self.InformationPanel`) (`self.InformationPanelTrackerIndex`) (`|FormatText` "{name} Status: Target Lost" (`KismetTextLibrary.Conv_StringToText` (`/Game/Blueprints/BP_ImageTrackerClass.GetTrackerName` (`self.ImageTrackerReference`))))))
    (:`then_2`
      ;[1 1 1] Hide tracked object
      (`self.SetActorHiddenInGame` (`self.TrackedObjectReference`) false))))

(fn `OnImageTargetUnreliable`
  (params (LastTrackedLocation :type "Vector Structure") (LastTrackedRotation :type "Rotator Structure") (NewUnreliableLocation :type "Vector Structure") (NewUnreliableRotation :type "Rotator Structure"))
  (locals (LocationOnUnreliable :type "Vector Structure") (RotationOnUnreliable :type "Rotator Structure"))
  (bind _trackedobjectreference (`self.TrackedObjectReference`))
  (if (`/Game/Blueprints/BP_ImageTrackerClass.GetUseUnreliablePose` (`self.ImageTrackerReference`))
    (`|ExecutionSequence`
      (:`then_0`
        ;[1 1 1] Determine location/rotation to use when tracking is unreliable
        (if (`self.UseUnreliableTransformData`)
          (set `local.LocationOnUnreliable` (`local.NewUnreliableLocation`))
          (set `local.RotationOnUnreliable` (`local.NewUnreliableRotation`))
          (else
            (set `local.LocationOnUnreliable` (`local.LastTrackedLocation`))
            (set `local.RotationOnUnreliable` (`local.LastTrackedRotation`)))))
      (:`then_1`
        (`|ExecutionSequence` :!label _label
          (:`then_0`
            (set `self.TrackingStatus` "NewEnumerator2"))
          (:`then_1`
            ;[1 1 1] Change text based on tracking state
            (`/Game/Examples/Blueprints/Utility/InformationPanel.SetTextAtIndex` (`self.InformationPanel`) (`self.InformationPanelTrackerIndex`) (`|FormatText` "{name} Status: Target Found (Unreliable)" (`KismetTextLibrary.Conv_StringToText` (`/Game/Blueprints/BP_ImageTrackerClass.GetTrackerName` (`self.ImageTrackerReference`))))))
          (:`then_2`
            ;[1 1 1] Move tracked object to tracking location
            (`self.K2_SetActorLocationAndRotation` _trackedobjectreference (`local.LocationOnUnreliable`) (select `bool` (`self.RotateTrackedObject`) :`false` (`self.K2_GetActorRotation` _trackedobjectreference) :`true` (`local.RotationOnUnreliable`)) false false))
          (:`then_3`
            ;[1 1 1] Set tracked object visibility based on flag
            (`self.SetActorHiddenInGame` (not (`/Game/Blueprints/BP_ImageTrackerClass.GetUseUnreliablePose` (`self.ImageTrackerReference`))))))))
    (else
      (goto _label))))

(fn `UpdateViewModeText`
  (`/Game/Examples/Blueprints/Utility/InformationPanel.SetTextAtIndex` (`self.InformationPanel`) 2 (`|FormatText` "View Mode: {mode}" (select `/Game/Examples/Enums/E_ImageTrackingVisualMode` (`/Game/Examples/Blueprints/Visualizers/ImageTracking/BP_DeepSeaVisualizer.GetCurrentViewMode` (`self.VisualizerReference`)) :`NewEnumerator0` "All" :`NewEnumerator1` "AxisOnly" :`NewEnumerator2` "TrackingCubeOnly" :`NewEnumerator3` "DemoOnly" :!type "Text"))))

(fn `UserConstructionScript`)